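; Flippit conversational avatar: overlapping it opens a WebSocket chat session and keeps it facing the player until they leave.
; Player input comes from a chat widget or from microphone recordings transcribed by OpenAI, gated by SendMessage.
; Replies fill chat widgets, while numbered MP3s are runtime-imported into an array for sequential voice playback.
; Received keys drive timed emote flags or AI movement to a named level actor.
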(event Custom|streamanimation
  (bind _animationkeys (Variables|Default|GetanimationKeys))
  ;[1 1 1] Emotes
  (Utilities|FlowControl|Sequence
    (:then_0
      (Variables|Default|Setdancing (Utilities|Enum|Equal(Enum) _animationkeys "Dancing")))
    (:then_1
      (Variables|Default|SetMagic (Utilities|Enum|Equal(Enum) _animationkeys "Magic")))
    (:then_2
      (Variables|Default|SetTalking (Utilities|Enum|Equal(Enum) _animationkeys "Talking")))
    (:then_3
      (Variables|Default|SetAngry (Utilities|Enum|Equal(Enum) _animationkeys "Angry")))
    (:then_4
      (Variables|Default|SetSinging (Utilities|Enum|Equal(Enum) _animationkeys "Singing")))
    (:then_5
      (Variables|Default|SetBragging (Utilities|Enum|Equal(Enum) _animationkeys "Bragging")))
    (:then_6
      (Variables|Default|SetAfraid (Utilities|Enum|Equal(Enum) _animationkeys "Afraid")))
    (:then_7
      (Variables|Default|SetExcited (Utilities|Enum|Equal(Enum) _animationkeys "Excited")))
    (:then_8
      (Variables|Default|SetGreetings (Utilities|Enum|Equal(Enum) _animationkeys "Greetings")))
    (:then_9
      (Variables|Default|SetSearching (Utilities|Enum|Equal(Enum) _animationkeys "Searching")))
    (:then_10
      (Variables|Default|SetShy (Utilities|Enum|Equal(Enum) _animationkeys "Shy")))
    (:then_11
      (Variables|Default|SetSurprised (Utilities|Enum|Equal(Enum) _animationkeys "Surprised")))
    (:then_12
      (Variables|Default|SetLevitating (Utilities|Enum|Equal(Enum) _animationkeys "Levitating"))))
  (bind _returnvalue (Class|FlippitCharacter|AssignAnimationtoString "Talking" "/Flippit/animation/Emotes/Talking__2_.Talking__2_" "Bragging" "/Flippit/animation/Emotes/Yelling.Yelling" "Dancing" "/ReadyPlayerMe/Character/Fullbody/Animations/Silly_Dancing.Silly_Dancing" "Afraid" "/Flippit/animation/Emotes/scared.scared" "Angry" "/Flippit/animation/Emotes/Angry_Point.Angry_Point" "Excited" "/Flippit/animation/Emotes/Clapping.Clapping" "Greetings" "/Flippit/animation/Emotes/Standing_Greeting.Standing_Greeting" "Singing" "/Flippit/animation/Emotes/Singing.Singing" "Magic" "/Flippit/animation/Emotes/Magic.Magic" "Searching" "/Flippit/animation/Emotes/Searching_Files_High.Searching_Files_High" "Shy" "/Flippit/animation/Emotes/Bashful.Bashful" "Surprised" "/Flippit/animation/Emotes/Reacting.Reacting" "Levitating" "/Flippit/animation/Emotes/Levitating.Levitating" _animationkeys))
  (Utilities|FlowControl|Delay (Animation|GetPlayLength _returnvalue))
  (Utilities|FlowControl|Sequence
    (:then_0
      (Variables|Default|Setdancing false))
    (:then_1
      (Variables|Default|SetMagic false))
    (:then_2
      (Variables|Default|SetTalking false))
    (:then_3
      (Variables|Default|SetAngry false))
    (:then_4
      (Variables|Default|SetSinging false))
    (:then_5
      (Variables|Default|SetBragging false))
    (:then_6
      (Variables|Default|SetAfraid false))
    (:then_7
      (Variables|Default|SetExcited false))
    (:then_8
      (Variables|Default|SetGreetings false))
    (:then_9
      (Variables|Default|SetSearching false))
    (:then_10
      (Variables|Default|SetShy false))
    (:then_11
      (Variables|Default|SetSurprised false))
    (:then_12
      (Variables|Default|SetLevitating false))))

(event Custom|TTS
  ;[1 1 1] TTS
  (if (Variables|Default|GetUseVoice)
    (Class|FlippitCharacter|PlaySoundsSequentially)))

(event Custom|CustomEvent_5
  (params (Importer :type Runtime%20Audio%20Importer%20Library%20Object%20Reference) (ImportedSoundWave :type Imported%20Sound%20Wave%20Object%20Reference) (Status :type ERuntimeImportStatus%20Enum :default "SuccessfulImport"))
  ;[1 1 1] TTS
  (Variables|Default|SetImporter 0)
  (Utilities|Array|AddUnique (Variables|Default|GetSoundWaveArray) ImportedSoundWave)
  (Math|Integer|IncrementInt (Variables|Default|GetJ)))

(event Custom|Pressed
  ;[1 1 1] Speech To Text
  (if (Variables|Default|GetUseMicrophone)
    (if (Variables|Default|GetIn%20the%20Zone)
      (Variables|Default|SetJ 0)
      (CameraShake|Start (Variables|Default|GetAudioCapture))
      (if (Variables|Default|Getenabled)
        (Class|AudioMixerBlueprintLibrary|StartRecordingOutput 1e+01 (Variables|Default|GetSubmix%20to%20Record))))))

(event Custom|Released
  ;[1 1 1] Speech To Text
  (if (Variables|Default|GetUseMicrophone)
    (if (Variables|Default|GetIn%20the%20Zone)
      (Audio|Components|Audio|Stop (Variables|Default|GetAudioCapture))
      (if (Variables|Default|Getenabled)
        (Class|AudioMixerBlueprintLibrary|StopRecordingOutput "WavFile" (Variables|Default|GetFileName) "" (Variables|Default|GetSubmix%20to%20Record) 0)
        (Utilities|FlowControl|Delay 0.2)
        (bind _transcription (|OpenAICallTranscriptions (Variables|Default|GetFileName))
          (:Finished
            (if (not (Utilities|Array|IsEmpty _transcription))
              (if (Variables|Default|GetUseText)
                (bind _returnvalue (UserInterface|CreateWidget "/Flippit/Blueprints/Chat_Text.Chat_Text_C" 0 (Utilities|Text|FormatText "{Sender } :{Text}" (Variables|/Flippit/Blueprints/BP_ChatUI.BP_ChatUI_C|Getnom (stale Collision|EventActorBeginOverlap _returnvalue)) _transcription)))
                (Widget|Panel|AddChild (Variables|/Flippit/Blueprints/BP_ChatUI.BP_ChatUI_C|GetChatLog (stale Collision|EventActorBeginOverlap _returnvalue)) _returnvalue)
                (Class|ScrollBox|ScrolltoEnd (Variables|/Flippit/Blueprints/BP_ChatUI.BP_ChatUI_C|GetChatLog (stale Collision|EventActorBeginOverlap _returnvalue))))
              (if (Variables|Default|GetSendMessage)
                (Class|FlippitCharacter|SendChatMessage _transcription)
                (if (Variables|Default|GetUseText)
                  ;[1 1 1] Interacte with avatar
                  (bind _returnvalue_2 (UserInterface|CreateWidget "/Flippit/Blueprints/Chat_Reply.Chat_Reply_C"))
                  (Widget|Panel|AddChild (Variables|/Flippit/Blueprints/BP_ChatUI.BP_ChatUI_C|GetChatLog (stale Collision|EventActorBeginOverlap _returnvalue)) _returnvalue_2)
                  (Class|ScrollBox|ScrolltoEnd (Variables|/Flippit/Blueprints/BP_ChatUI.BP_ChatUI_C|GetChatLog (stale Collision|EventActorBeginOverlap _returnvalue))))))))))))

(event Custom|Done
  ;[1 1 1] Interacte with avatar
  (Variables|Default|SetSendMessage true))

(event Custom|OnClicked_Event_0
  ;[1 1 1] Interacte with avatar
  (if (Variables|Default|GetSendMessage)
    (Variables|Default|SetJ 0)
    (if (not (Utilities|Text|TextIsEmpty (Variables|/Script/UMG.EditableTextBox|GetText (Variables|/Flippit/Blueprints/BP_ChatUI.BP_ChatUI_C|GetChatEntry (stale Collision|EventActorBeginOverlap _returnvalue)))))
      (bind _returnvalue (UserInterface|CreateWidget "/Flippit/Blueprints/Chat_Text.Chat_Text_C" 0 (Utilities|Text|FormatText "{Sender } :{Text}" (Variables|/Flippit/Blueprints/BP_ChatUI.BP_ChatUI_C|Getnom (stale Collision|EventActorBeginOverlap _returnvalue)) (Variables|/Script/UMG.EditableTextBox|GetText (Variables|/Flippit/Blueprints/BP_ChatUI.BP_ChatUI_C|GetChatEntry (stale Collision|EventActorBeginOverlap _returnvalue))))))
      (Widget|Panel|AddChild (Variables|/Flippit/Blueprints/BP_ChatUI.BP_ChatUI_C|GetChatLog (stale Collision|EventActorBeginOverlap _returnvalue)) _returnvalue)
      (Class|ScrollBox|ScrolltoEnd (Variables|/Flippit/Blueprints/BP_ChatUI.BP_ChatUI_C|GetChatLog (stale Collision|EventActorBeginOverlap _returnvalue)))
      (Class|FlippitCharacter|SendChatMessage (Utilities|String|ToString(Text) (Variables|/Script/UMG.EditableTextBox|GetText (Variables|/Flippit/Blueprints/BP_ChatUI.BP_ChatUI_C|GetChatEntry (stale Collision|EventActorBeginOverlap _returnvalue)))))
      (Variables|/Script/UMG.EditableTextBox|SetText (Variables|/Flippit/Blueprints/BP_ChatUI.BP_ChatUI_C|GetChatEntry (stale Collision|EventActorBeginOverlap _returnvalue)) "")
      (bind _returnvalue_2 (UserInterface|CreateWidget "/Flippit/Blueprints/Chat_Reply.Chat_Reply_C"))
      (Widget|Panel|AddChild (Variables|/Flippit/Blueprints/BP_ChatUI.BP_ChatUI_C|GetChatLog (stale Collision|EventActorBeginOverlap _returnvalue)) _returnvalue_2)
      (Class|ScrollBox|ScrolltoEnd (Variables|/Flippit/Blueprints/BP_ChatUI.BP_ChatUI_C|GetChatLog (stale Collision|EventActorBeginOverlap _returnvalue))))))

(event Custom|Import
  ;[1 1 1] TTS
  (bind _returnvalue (Class|RuntimeAudioImporterLibrary|CreateRuntimeAudioImporter))
  (bind _output_get (Variables|Default|SetImporter _returnvalue))
  (EventDispatchers|BindEventtoOnResult _output_get (delegate Custom|CustomEvent_5))
  (Class|RuntimeAudioImporterLibrary|ImportAudiofromFile (Variables|Default|GetImporter) (Utilities|String|Append (Class|KismetSystemLibrary|GetProjectDirectory) "Saved/Sounds/MyAudio" (Utilities|String|ToString(Integer) (Variables|Default|GetJ)) ".mp3") "Auto"))

(event Custom|message
  ;[1 1 1] Interacte with avatar
  (if (Variables|Default|GetUseText)
    (Variables|Default|SetIn%20the%20Zone true)
    (Variables|/Flippit/Blueprints/Chat_Reply.Chat_Reply_C|SetChatReply (stale Custom|Released _returnvalue_2) (Utilities|Text|FormatText "{Sender}:{Text}" (Variables|Default|GetcharacterName) (Variables|Default|GetMessagesrecieved)))
    (Variables|Default|SetSendMessage false)))

(event Custom|Face
  ;[1 1 1] Face The Player
  (if (Variables|Default|Getshould%20rotate)
    (Transformation|SetActorRotation (Math|Rotator|MakeRotator 0.0 0.0 (.yaw (Math|Interpolation|RInterpTo (Transformation|GetActorRotation) (Math|Rotator|FindLookatRotation (Transformation|GetActorLocation) (Transformation|GetActorLocation (Variables|Default|GetCHarRef))) (Utilities|Time|GetWorldDeltaSeconds) 2e+01))))
    (Utilities|FlowControl|Delay 0.051)
    (CallFunction|Face)))

(event Custom|Streamwalking
  ;[1 1 1] Navigation
  (Variables|Default|Setshould%20rotate false)
  (Utilities|FlowControl|Delay 0.2)
  (Class|FlippitCharacter|LogNamesOfAllObjectsinLevel)
  (bind _returnvalue (Class|FlippitCharacter|GetLocationOfActorbyName (Variables|Default|Getdestinationkey)))
  (AI|AIMoveTo self _returnvalue 0 1e+01 false))

(event EventBeginPlay
  ;[1 1 1] Speech To Text
  (bind _outdevices (Class|MediaBlueprintFunctionLibrary|EnumerateAudioCaptureDevices -1))
  (Variables|Default|Setenabled (>= (Utilities|Array|Length _outdevices) 1))
  (if (Variables|Default|Getenabled)
    (Class|OpenAIUtils|SetOpenAIApiKey (Variables|Default|GetOpenAIKey))))

(event Collision|EventActorBeginOverlap
  (params (OtherActor :type Actor%20Object%20Reference))
  ;[1 1 1] Interacte with avatar
  (Class|FlippitCharacter|OnPlayerEnterInteractionZone)
  (Variables|Default|SetIn%20the%20Zone true)
  (Class|FlippitCharacter|EstablishWebSocketConnection)
  (if (Variables|Default|GetUseText)
    (bind _returnvalue (UserInterface|CreateWidget "/Flippit/Blueprints/BP_ChatUI.BP_ChatUI_C" 0 "Me"))
    (UserInterface|Viewport|AddtoViewport _returnvalue 0)
    (EventDispatchers|AssignOnClicked (Variables|/Flippit/Blueprints/BP_ChatUI.BP_ChatUI_C|GetButton_0 _returnvalue) (delegate Custom|OnClicked_Event_0)))
  ;[1 1 1] Face The Player
  (Variables|Default|Setshould%20rotate true)
  (bind _asbp_third_person_character (Utilities|Casting|CastToBP_ThirdPersonCharacter (Game|GetPlayerCharacter 0)))
  (Variables|Default|SetCHarRef _asbp_third_person_character)
  (CallFunction|Face))

(event Collision|EventActorEndOverlap
  (params (OtherActor :type Actor%20Object%20Reference))
  ;[1 1 1] End Interaction with avatar
  (Class|FlippitCharacter|CloseWebSocketConnection)
  (Viewport|RemoveAllWidgets)
  (Variables|Default|Setshould%20rotate false)
  (Variables|Default|SetIn%20the%20Zone false))

(fn ConstructionScript)